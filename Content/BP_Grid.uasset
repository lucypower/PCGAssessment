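; BP_Grid is an actor for a random two-state cell grid, with a work-in-progress neighbour check.
; MakeGrid spawns cube mesh components by row and column, using Density to pick black or white and recording booleans in OriginalCells.
; IterateGrid only logs each cell's next-in-row neighbour, treating edges as filled; RemoveGrid clears the meshes.
; BeginPlay enables input for a P-key debug print; MakeGrid calls in both graphs are disconnected.
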(event EventBeginPlay
  (Input|EnableInput (Game|GetPlayerController 0)))

(event Input|KeyboardEvents|P
  (params (Key :type Key%20Structure))
  (:Pressed
    (for _array_element (Variables|Default|GetOriginalCells)
      (Development|PrintString (Utilities|String|ToString(Boolean) _array_element)))))

(fn ConstructionScript)

(fn MakeGrid
  (Variables|Default|SetArrayIndex 0)
  (for _index (range 0 (- (Variables|Default|GetRows) 1))
    (for _index_2 (range 0 (- (Variables|Default|GetColumns) 1))
      (bind _returnvalue (AddComponent|AddStaticMeshComponent false (Math|Transform|MakeTransform (Math|Vector|MakeVector (* _index_2 (Variables|Default|GetCellSize)) (* _index (Variables|Default|GetCellSize)) 0.0) "0, 0, 0" "1.000000,1.000000,1.000000")))
      (Utilities|Array|Add (Variables|Default|GetStaticMesh) _returnvalue)
      (bind _output_get (Variables|Default|SetRandomInt (Math|Random|RandomIntegerinRange 0 100)))
      (Utilities|String|LogString (Utilities|String|ToString(Integer) _output_get))
      (if (<= _output_get (Variables|Default|GetDensity))
        (Utilities|String|LogString "true black ")
        (Components|StaticMesh|SetStaticMesh _returnvalue "/Game/StarterContent/Shapes/Shape_BlackCube.Shape_BlackCube")
        (Utilities|Array|SetArrayElem (Variables|Default|GetOriginalCells) (Variables|Default|GetArrayIndex) true true)
        (else
          (Utilities|String|LogString "false white")
          (Components|StaticMesh|SetStaticMesh _returnvalue "/Game/StarterContent/Shapes/Shape_Cube.Shape_Cube")
          (Utilities|Array|SetArrayElem (Variables|Default|GetOriginalCells) (Variables|Default|GetArrayIndex) false true)))
      (Math|Integer|IncrementInt (Variables|Default|GetArrayIndex)))))

(fn RemoveGrid
  (for _array_element (Variables|Default|GetStaticMesh)
    (Components|DestroyComponent _array_element))
  (Utilities|Array|Clear (Variables|Default|GetStaticMesh)))

(fn IterateGrid
  (for (_ _array_index) (Variables|Default|GetOriginalCells)
    (if (> (+ _array_index 1) (- (Utilities|Array|Length (Variables|Default|GetOriginalCells)) 1))
      (Utilities|String|LogString "true" :!label _label)
      (elif (== (Math|Integer|%(Integer) (+ _array_index 1) (Variables|Default|GetColumns)) 0)
        (goto _label)
        (elif (Utilities|Array|Get(acopy) (Variables|Default|GetOriginalCells) (+ _array_index 1))
          (goto _label)
          (else
            (Utilities|String|LogString "false")))))))