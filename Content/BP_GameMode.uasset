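; BP_GameMode is a game mode that sets up the settings UI for a grid at BeginPlay.
; It creates and shows BP_Widget, switches input to UI-only focused on it, and enables the mouse cursor.
; It then finds the BP_Grid actor and copies its Rows, Columns and Density values into the widget's text fields.
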(event EventBeginPlay
  (bind _returnvalue (Game|GetPlayerController 0))
  (bind _returnvalue_2 (UserInterface|CreateWidget "/Game/BP_Widget.BP_Widget_C"))
  (Variables|/Game/BP_Widget.BP_Widget_C|SetSpawn%20Transform _returnvalue_2 (Variables|/Game/BP_Widget.BP_Widget_C|GetSpawn%20Transform _returnvalue_2))
  (UserInterface|Viewport|AddtoViewport _returnvalue_2 0)
  (Input|SetInputModeUIOnly _returnvalue _returnvalue_2 "DoNotLock" false)
  (Variables|/Script/Engine.PlayerController|SetbShowMouseCursor _returnvalue true)
  (bind _returnvalue_3 (Actor|GetActorOfClass "/Game/BP_Grid.BP_Grid_C"))
  (Rendering|Components|TextRender|SetText (Variables|/Game/BP_Widget.BP_Widget_C|GetRowsText _returnvalue_2) (Utilities|Text|ToText(Integer) (Variables|/Game/BP_Grid.BP_Grid_C|GetRows _returnvalue_3)))
  (Rendering|Components|TextRender|SetText (Variables|/Game/BP_Widget.BP_Widget_C|GetColumnsText _returnvalue_2) (Utilities|Text|ToText(Integer) (Variables|/Game/BP_Grid.BP_Grid_C|GetColumns _returnvalue_3)))
  (Rendering|Components|TextRender|SetText (Variables|/Game/BP_Widget.BP_Widget_C|GetDensityText _returnvalue_2) (Utilities|Text|ToText(Integer) (Variables|/Game/BP_Grid.BP_Grid_C|GetDensity _returnvalue_3))))

(fn ConstructionScript)