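; Room spawner actor that randomly scatters room actors over a flat area when triggered from the UI.
; On BeginPlay it binds SpawnRooms to a dispatcher on the first BP_Widget found.
; For each ActorsToSpawn class, SpawnRooms destroys existing actors, then spawns a random number of randomly picked classes, so later passes can remove earlier spawns.
; BossRoom is an unfinished stub whose binding never runs, and RoomsSpawned is recorded but unused.
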(event Custom|SpawnRooms
  (bind _actorstospawn (Variables|Default|GetActorsToSpawn))
  (for _index (range 0 (Utilities|Array|Length _actorstospawn))
    (bind _outactors (Actor|GetAllActorsOfClass (Utilities|Array|Get(acopy) _actorstospawn _index)))
    (Actor|DestroyActor _outactors)
    (for _index_2 (range 0 (Math|Random|RandomInteger 15))
      (bind _output_get (Variables|Default|SetRoomSpawnLocation (Math|Random|RandomPointinBoundingBox "0.000000,0.000000,10.000000" "1000.000000,1000.000000,0.000000")))
      (bind _returnvalue (Game|SpawnActorfromClass (.OutItem (Utilities|Array|Random (Variables|Default|GetActorsToSpawn))) (Math|Conversions|ToTransform(Vector) _output_get) "AdjustIfPossibleButDontSpawnIfColliding" "MultiplyWithRoot" 0 0))
      (Utilities|Array|Add (Variables|Default|GetRoomsSpawned) _returnvalue))))

(event Custom|BossRoom
  (if (Variables|/Game/BP_Widget.BP_Widget_C|GetBossRoom (Variables|Default|GetWidgetReference))
    _))

(event EventBeginPlay
  (bind _foundwidgets (Widget|GetAllWidgetsOfClass "/Game/BP_Widget.BP_Widget_C" true))
  (EventDispatchers|BindEventtoSpawnRoomDispatcher (Utilities|Array|Get(acopy) _foundwidgets) (delegate Custom|SpawnRooms)))

(fn ConstructionScript)